(event Custom|Create
  (Class|PythonScriptLibrary|ExecutePythonCommand (Utilities|String|Append (Utilities|String|Append (Utilities|String|Append (Utilities|String|Append (Utilities|String|Append (Utilities|String|Append "import importlib, song_lights; importlib.reload(song_lights); song_lights.create('" (Class|KismetSystemLibrary|GetPathName (Variables|Song|GetSong))) "', camera='") (Class|KismetSystemLibrary|GetPathName (Variables|Song|GetCamera))) "', fps=") (Utilities|String|ToString(Integer) (Variables|Song|GetFPS))) ")")))

(event Custom|SetupRig
  (bind _rigorigin (Variables|StarterRig|GetRigOrigin))
  (bind (_x _y _z) (Math|Vector|BreakVector _rigorigin))
  (Class|PythonScriptLibrary|ExecutePythonCommand (Utilities|String|Append (Utilities|String|Append (Utilities|String|Append (Utilities|String|Append (Utilities|String|Append (Utilities|String|Append "import importlib, song_lights; importlib.reload(song_lights); song_lights.setup_rig_for_director(origin=(" (Utilities|String|ToString(Float) _x)) ",") (Utilities|String|ToString(Float) _y)) ",") (Utilities|String|ToString(Float) _z)) "))")))

(event EventBeginPlay)

(event Collision|EventActorBeginOverlap
  (params (OtherActor :type Actor%20Object%20Reference)))

(event EventTick
  (params (DeltaSeconds :type Float%20%28single-precision%29)))

(fn ConstructionScript)